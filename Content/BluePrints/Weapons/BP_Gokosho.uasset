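; BP_Gokosho is a destructible homing projectile that deals damage to the player on overlap, then destroys itself.
; A timeline played from Tick scales forward movement along MoveDirection with a speed curve while the mesh spins.
; A timeline event track switches on homing, which gradually lerps rotation toward a point just ahead of the player.
; Each damage event removes one HP, and at zero it explodes and is destroyed.
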(event EventBeginPlay
  (Variables|Default|SetPlayer (Class|MyBlueprintFunctionLibrary|FindUniqueActorOfClass "/Script/SpecterFront.PlayerCharacter")))

(event EventTick
  (params (DeltaSeconds :type Float%20%28single-precision%29))
  (bind _player (Variables|Default|GetPlayer))
  (bind _staticmesh (Variables|Default|GetStaticMesh))
  (bind _speed (Timeline|SpeedTimeLine Play)
    (:Update
      (Utilities|FlowControl|Sequence
        (:then_0
          (Transformation|AddActorLocalOffset (* (Variables|Default|GetMoveDirection) (* _speed DeltaSeconds (Variables|Default|GetSpeed))) false false)
          (Utilities|IsValid _staticmesh
            (:Is%20Valid
              (Transformation|AddLocalRotation _staticmesh (Math|Rotator|MakeRotator 0.0 (* (Utilities|Time|GetWorldDeltaSeconds) 6e+01) 0.0) false false))))
        (:then_1
          (if (Variables|Default|GetIsPlayerFollowing)
            (Transformation|SetActorRotation (Math|Rotator|Lerp(Rotator) (Transformation|GetActorRotation) (Math|Rotator|FindLookatRotation (Transformation|GetActorLocation) (+ (Transformation|GetActorLocation _player) (* (Transformation|GetActorForwardVector _player) 5e+01))) 0.06 true))))))
    (:PlayerForrowing
      (Variables|Default|SetIsPlayerFollowing true))))

(event Collision|EventActorBeginOverlap
  (params (OtherActor :type Actor%20Object%20Reference))
  (if (Actor|ActorHasTag OtherActor "Player")
    (bind _asbp_player (Utilities|Casting|CastToBP_Player OtherActor))
    (Class|PlayerCharacter|OnDamage _asbp_player 1e+02 0 self)
    (Actor|DestroyActor)))

(event Game|Damage|EventAnyDamage
  (params (Damage :type Float%20%28single-precision%29) (DamageType :type Damage%20Type%20Object%20Reference) (InstigatedBy :type Controller%20Object%20Reference) (DamageCauser :type Actor%20Object%20Reference))
  (bind _output_get (Variables|Default|SetHP (- (Variables|Default|GetHP) 1)))
  (if (<= _output_get 0)
    (Effects|SpawnEmitteratLocation "/Game/Effects/P_MyExplosion.P_MyExplosion" (Transformation|GetActorLocation))
    (Actor|DestroyActor)))

(fn ConstructionScript)