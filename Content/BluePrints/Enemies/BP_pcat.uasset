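; BP_pcat is an enemy Blueprint that pursues the player and damages them on contact.
; Its Attack function rotates it toward the player pawn and has its AI controller move to that pawn, with a wide acceptance radius.
; Overlapping an actor tagged Player calls OnDamage on the unique BP_Player, passing Power as damage.
; A manual movement calculation remains unused, and nothing here calls Attack.
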(event Collision|EventActorBeginOverlap
  (params (OtherActor :type Actor%20Object%20Reference))
  (if (Actor|ActorHasTag OtherActor "Player")
    (Class|PlayerCharacter|OnDamage (Class|MyBlueprintFunctionLibrary|FindUniqueActorOfClass "/Game/BluePrints/Player/BP_Player.BP_Player_C") (Variables|Default|Getpower) (Pawn|GetController) self)))

(fn ConstructionScript
  (|CallParentFunction))

(fn Attack
  (params (deltaTime :type Float%20%28single-precision%29))
  (Transformation|SetActorRotation (Math|Rotator|FindLookatRotation (Transformation|GetActorLocation) (Transformation|GetActorLocation (Game|Player|GetPlayerPawn 0))))
  (AI|Navigation|MovetoActor (.AsAIController (Utilities|Casting|CastToAIController (Pawn|GetController))) (Game|Player|GetPlayerPawn 0) 5e+02 true true))