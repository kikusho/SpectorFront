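; BP_Daibutu is a boss enemy with an HP bar, taking damage only while ShowHPBar is set.
; Tick watches that flag to toggle the bar and start a looping missile volley.
; MisileShot fans missiles upward from VectorField, doubling from two to four below half HP.
; On death it removes the bar, kills every other BP_BaseEnemy and damages all BP_Gokosho actors.
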(event EventBeginPlay
  (Utilities|FlowControl|Sequence
    (:then_0
      (bind _returnvalue (UserInterface|CreateWidget "/Game/BluePrints/UI/WBP_HPBar.WBP_HPBar_C" 0 self))
      (Variables|Default|SetHPBar _returnvalue))
    (:then_1
      (Utilities|FlowControl|Delay 5.0)
      (Utilities|FlowControl|Gate true) ; enters at Open
    )))

(event Collision|EventActorBeginOverlap
  (params (OtherActor :type Actor%20Object%20Reference))
  (Utilities|FlowControl|Gate true
    (:Exit
      (Utilities|Casting|CastToBP_Player OtherActor))))

(event EventOnDamage
  (params (damage :type Float%20%28single-precision%29) (instigatedBy :type Controller%20Object%20Reference) (damageCauser :type Actor%20Object%20Reference))
  (if (Variables|Default|GetShowHPBar)
    (|CallParentFunction damage instigatedBy damageCauser)))

(event EventTick
  (params (DeltaSeconds :type Float%20%28single-precision%29))
  (bind _showhpbar (Variables|Default|GetShowHPBar))
  ;[1 1 1] HPバーの表示を切り替える
  (if (Math|Boolean|NotEqual(Boolean) _showhpbar (Variables|Default|GetOldShowHPBar))
    (Utilities|FlowControl|Sequence
      (:then_0
        (Utilities|IsValid (Variables|Default|GetHPBar)
          (:Is%20Not%20Valid
            (bind _returnvalue (UserInterface|CreateWidget "/Game/BluePrints/UI/WBP_HPBar.WBP_HPBar_C" 0 self))
            (Variables|Default|SetHPBar _returnvalue))))
      (:then_1
        (if _showhpbar
          (UserInterface|Viewport|AddtoViewport (Variables|Default|GetHPBar) 0)
          (Utilities|FlowControl|Sequence
            (:then_0
              ;[1 1 1] ミサイル発射
              (if (< (Class|BaseEnemy|GetHp) (/ (Class|BaseEnemy|GetMaxHp) 2.0)) :!label _label
                (CallFunction|MisileShot 4)
                (else
                  (CallFunction|MisileShot 2)))
              (Utilities|FlowControl|Delay (Variables|Default|GetMisileInterval))
              (goto _label))
            (:then_1
              _))
          (else
            (Widget|RemovefromParent (Variables|Default|GetHPBar))))
        (Variables|Default|SetOldShowHPBar _showhpbar)))))

(event EventOnDeath
  (params (instigatedBy :type Controller%20Object%20Reference) (damageCauser :type Actor%20Object%20Reference))
  (|CallParentFunction instigatedBy damageCauser)
  (Widget|RemovefromParent (Variables|Default|GetHPBar))
  (bind _outactors (Actor|GetAllActorsOfClass "/Game/BluePrints/Enemies/BP_BaseEnemy.BP_BaseEnemy_C"))
  (for _array_element _outactors
    (Utilities|IsValid _array_element
      (:Is%20Valid
        (if (!= _array_element self)
          (Class|BaseEnemy|Kill _array_element)))))
  (bind _outactors_2 (Actor|GetAllActorsOfClass "/Game/BluePrints/Weapons/BP_Gokosho.BP_Gokosho_C"))
  (for _array_element_2 _outactors_2
    (Game|Damage|ApplyDamage _array_element_2 1e+02 0 0)))

(fn ConstructionScript)

(fn MisileShot
  (params (MisileCount :type Integer))
  (for _index (range 1 MisileCount)
    (bind _returnvalue (Game|SpawnActorfromClass (Variables|Default|GetMisileClass) (Math|Transform|MakeTransform (Transformation|GetWorldLocation (Variables|Default|GetVectorField)) (Math|Rotator|MakeRotator 0.0 9e+01 0.0) "1,1,1") "Undefined" 0 0))
    (Class|Actor|AddActorWorldRotation _returnvalue (Math|Rotator|MakeRotator (- (* _index (/ 1.8e+02 (Math|Conversions|ToFloat(Integer) (+ MisileCount 1)))) 9e+01) 0.0 0.0))))