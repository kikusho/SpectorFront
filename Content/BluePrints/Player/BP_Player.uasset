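; Player actor that rides on BP_PlayerCamera, handling shooting, damage and score hookup.
; BeginPlay attaches it to the camera and binds score changes to a debug print; after level transitions it also restores GameInstance's carried-over score into GameState.
; Firing deprojects the reticle to aim a spawned BP_Projectile, and landed hits spawn sparks, plus explosions on living BaseEnemy targets.
; Damage lowers HP through a DoOnce-and-Delay invincibility window and broadcasts the change.
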(event Custom|OnScoreChanged
  (params (NewScore :type Integer))
  (Development|PrintString (Utilities|String|ToString(Integer) NewScore)))

(event Custom|PostLevelTransition
  (bind _returnvalue (Class|MyBlueprintFunctionLibrary|FindUniqueActorOfClass "/Game/BluePrints/Player/BP_PlayerCamera.BP_PlayerCamera_C"))
  (bind _score (Default|GetTakeOverScore (.AsBP%20Game%20Instance (Utilities|Casting|CastToBP_GameInstance (Game|GetGameInstance)))))
  (Default|SetScore (.AsBP%20Game%20State (Utilities|Casting|CastToBP_GameState (Game|GetGameState))) _score)
  (Utilities|IsValid _returnvalue
    (:Is%20Valid
      (Variables|Default|SetcameraComponent (Variables|/Game/BluePrints/Player/BP_PlayerCamera.BP_PlayerCamera_C|GetCamera _returnvalue))
      (Transformation|AttachActorToActor _returnvalue "None" "SnapToTarget" "SnapToTarget" "SnapToTarget" false)
      (EventDispatchers|BindEventtoScoreObservable (.AsBP%20Game%20State (Utilities|Casting|CastToBP_GameState (Game|GetGameState))) (delegate Custom|OnScoreChanged)))))

(event EventOnDamage
  (params (damage :type Float%20%28single-precision%29) (instigatedBy :type Controller%20Object%20Reference) (damageCauser :type Actor%20Object%20Reference))
  (Utilities|FlowControl|DoOnce false :!label _label
    (:Completed
      (bind _output_get (Variables|Default|Sethp (- (Variables|Default|Gethp) damage)))
      (Default|CallHpChangeDispatcher _output_get)
      (Utilities|FlowControl|Delay (Variables|Default|GetInvincibleTime))
      (goto _label Reset))))

(event EventOnFire
  (bind _returnvalue (Class|PlayerCharacter|GetReticleLocation))
  (bind _returnvalue_2 (Transformation|GetActorLocation))
  (bind _returnvalue_3 (Game|GetPlayerController 0))
  (bind (_worldposition _worlddirection) (Class|GameplayStatics|DeprojectScreentoWorld _returnvalue_3 _returnvalue))
  (|CallParentFunction)
  (Game|SpawnActorfromClass "/Game/BluePrints/Weapons/BP_Projectile.BP_Projectile_C" (Math|Transform|MakeTransform (+ (+ _returnvalue_2 (* _worlddirection 5.0)) "0, 0,-50.000000") (Math|Rotator|FindLookatRotation _returnvalue_2 (+ _worldposition (* _worlddirection 1e+02))) "1,1,1") "Undefined" 0 0))

(event EventBeginPlay
  (bind _returnvalue (Class|MyBlueprintFunctionLibrary|FindUniqueActorOfClass "/Game/BluePrints/Player/BP_PlayerCamera.BP_PlayerCamera_C"))
  (EventDispatchers|AssignPostLevelTransitionDelegate (.AsBP%20Game%20Instance (Utilities|Casting|CastToBP_GameInstance (Game|GetGameInstance))) (delegate Custom|PostLevelTransition))
  (Utilities|IsValid _returnvalue
    (:Is%20Valid
      (Variables|Default|SetcameraComponent (Variables|/Game/BluePrints/Player/BP_PlayerCamera.BP_PlayerCamera_C|GetCamera _returnvalue))
      (Transformation|AttachActorToActor _returnvalue "None" "SnapToTarget" "SnapToTarget" "SnapToTarget" false)
      (EventDispatchers|BindEventtoScoreObservable (.AsBP%20Game%20State (Utilities|Casting|CastToBP_GameState (Game|GetGameState))) (delegate Custom|OnScoreChanged)))))

(event EventOnLanding
  (params (hit :type Hit%20Result%20Structure))
  (Effects|SpawnEmitteratLocation "/Game/Effects/P_Spark.P_Spark" (.location hit) (Math|Rotator|FindLookatRotation (Math|Vector|MakeVector 0.0 0.0 0.0) (.normal hit)))
  (bind _asbase_enemy (Utilities|Casting|CastToBaseEnemy (.hitactor hit)))
  (if (> (Class|BaseEnemy|GetHp _asbase_enemy) 0.0)
    (Effects|SpawnEmitteratLocation "/Game/Effects/P_SmoleExplosion.P_SmoleExplosion" (.location hit))))

(fn ConstructionScript)