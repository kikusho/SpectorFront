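; BP_ActionPhase is a combat phase actor that runs enemy spawners one after another during a level sequence, optionally pausing the sequencer.
; Each spawner's finish callback triggers the next and informs the player.
; Once spawners run out, a Tick gate waits until no enemies remain, unless ignorable, then after a delay resumes the sequencer and notifies the manager.
; Non-pausing phases also notify the manager shortly after starting.
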(event Custom|BeginActionPhase
  (params (ActionPhaseManager :type BP%20Action%20Phase%20Manager%20Object%20Reference) (Sequencer :type Level%20Sequence%20Actor%20Object%20Reference) (ActorContainer :type Actor%20Container%20Object%20Reference))
  (bind _sequenceplayer (Variables|/Script/LevelSequence.LevelSequenceActor|GetSequencePlayer Sequencer))
  ;[1 1 1] アクションフェーズ開始
  (Variables|Default|SetAllActors ActorContainer)
  (Variables|Default|SetManager ActionPhaseManager)
  (Utilities|FlowControl|Sequence ; アクションフェーズ開始時にスポーン制御を開始する
    (:then_0
      ;[1 1 1] 次のSpawnerを起動する
      (Utilities|ExecNextSpawner (Utilities|Struct|MakeFinishSpawn (delegate Custom|OnFinishSpawn))
        (:Completed
          (Utilities|FlowControl|Gate true) ; enters at Open
        )))
    (:then_1
      (if (Variables|ActionPhase|GetIsSequenceStop)
        (Sequencer|Player|Pause _sequenceplayer)
        (else
          (Utilities|FlowControl|Delay 0.2)
          (Default|OnActionEnd (Variables|Default|GetManager)))))))

(event Custom|OnFinishSpawn
  ;[1 1 1] 次のSpawnerを起動する
  (Utilities|ExecNextSpawner (Utilities|Struct|MakeFinishSpawn (delegate Custom|OnFinishSpawn))
    (:Completed
      (Utilities|FlowControl|Gate true) ; enters at Open
    )))

(event EventTick
  (params (DeltaSeconds :type Float%20%28single-precision%29))
  (|CallParentFunction DeltaSeconds)
  (Class|PlayerCharacter|TickActionPhase (Variables|Default|GetPlayer))
  (Utilities|FlowControl|Gate true :!label _label
    (:Exit
      (if (Variables|ActionPhase|GetIsIgnoreble)
        (Utilities|FlowControl|Delay (Variables|Default|GetLateWaitSeconds) :!label _label_2)
        (CallFunction|ResumeSequencer (Variables|/Script/LevelSequence.LevelSequenceActor|GetSequencePlayer (stale Custom|BeginActionPhase Sequencer))) ; シーケンサーを再開
        (goto _label Close)
        (else
          ;[1 1 1] 敵が全滅するまで待機
          (Utilities|IsValid (Variables|Default|GetCurrentSpawner)
            (:Is%20Not%20Valid
              (if (== (Class|AbstractEnemySpawner|GetSpawnedEnemyCount) 0)
                (goto _label_2)))))))))

(event EventBeginPlay
  (|CallParentFunction)
  (Variables|Default|SetPlayer (Class|MyBlueprintFunctionLibrary|FindUniqueActorOfClass "/Script/SpecterFront.PlayerCharacter")))

(fn ConstructionScript
  (Rendering|Components|TextRender|SetText (Variables|Default|GetText) (Utilities|Text|ToText(String) (Utilities|GetDisplayName self))))

(fn NextSpawn)

(fn ResumeSequencer
  (params (NewParam :type Level%20Sequence%20Player%20Object%20Reference))
  (if (Variables|ActionPhase|GetIsSequenceStop)
    (Audio|Components|Audio|Play NewParam))
  (Default|OnActionEnd (Variables|Default|GetManager)))